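; BP_CameraRig is a camera rig actor meant to show scanner state through a ScanLight color and a ScanBeam.
; ApplyState sets the light from GetColorForState and shows the beam only while Scanning, but always requests the Idle color.
; GetColorForState returns black because its per-state color switch is disconnected.
; BeginPlay only looks up BP_StateManager actors; the cast and OnStateChanged binding are unwired, and nothing here calls ApplyState.
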(event `self.ReceiveBeginPlay`
  (bind _outactors (`GameplayStatics.GetAllActorsOfClass` "/Game/CameraModule/Core/BP_StateManager.BP_StateManager_C")))

(fn `ApplyState`
  (params (NewState :type "EModuleState Enum" :default "Idle"))
  (bind _outcolor (`self.GetColorForState` "Idle"))
  (`LightComponent.SetLightColor` (`self.ScanLight`) _outcolor true)
  (if (`|EnumEquality` NewState "Scanning")
    (`SceneComponent.SetHiddenInGame` (`self.ScanBeam`) false false)
    (else
      (`SceneComponent.SetHiddenInGame` (`self.ScanBeam`) true false))))

(fn `GetColorForState`
  (params (InState :type "EModuleState Enum" :default "Idle"))
  (returns (OutColor :type "LinearColor Structure"))
  (return))

(fn `UserConstructionScript`)